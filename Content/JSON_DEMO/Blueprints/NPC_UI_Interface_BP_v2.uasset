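; Manager actor that links NPCs to a story screen widget and picks story branches based on each NPC's personality traits.
; It creates the hidden widget at BeginPlay, then opens it with an NPC and story node array, relaying NPC updates back.
; Next-node selection scores child options by matching trait names, inverting values for low NPC traits, and takes the highest.
; An older, non-working scoring function remains unused.
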(event `self.ReceiveBeginPlay`
  (`self.Interface_func_SetTraitEnums`)
  (`self.Interface_func_CreateMenu`))

(fn `Interface_func_CalculateAttractivenessToAdd`
  (params (Input_NPCTraitValue :type "Float (double-precision)") (Input_NodeTraitValue :type "Float (double-precision)"))
  (returns (Output_AttractivenessValueToAdd :type "Float (double-precision)"))
  (locals (Interface_tempVar_TempResult :type "Float (double-precision)"))
  (set `local.Interface_tempVar_TempResult` 0.0)
  (if (>= Input_NPCTraitValue 0.5)
    (set `local.Interface_tempVar_TempResult` (* Input_NPCTraitValue Input_NodeTraitValue))
    (else
      (set `local.Interface_tempVar_TempResult` (* (- 1.0 Input_NPCTraitValue) (- 1.0 Input_NodeTraitValue)))))
  (return (`local.Interface_tempVar_TempResult`)))

(fn `Interface_func_CreateMenu`
  (bind _returnvalue (`|CreateWidget` "/Game/JSON_DEMO/Widgets/UI_StoryScreen_WBP.UI_StoryScreen_WBP_C" (`GameplayStatics.GetPlayerController` 0)))
  (`UserWidget.AddToViewport` _returnvalue 0)
  (`Widget.SetVisibility` _returnvalue "Hidden")
  (set `self.Interface_var_MenuRef` _returnvalue)
  (`/Game/JSON_DEMO/Widgets/UI_StoryScreen_WBP.UI_func_SetInterfaceRef` _returnvalue self))

(fn `Interface_func_GetCurrentNode`
  (returns (NewParam :type "/Game/Structures/NPC_StoryNode_ArrayStructure Structure"))
  (return (`self.Interface_var_CurrentStoryNode`)))

(fn `Interface_func_GetCurrentNPC`
  (returns (outputNPCstructure :type "/Game/Structures/NPC_Structure Structure"))
  (return (`self.Interface_var_CurrentNPCArrayStructure`)))

(fn `Interface_func_GetIsTutorialBool`
  (returns (NewParam :type Boolean))
  (return (`self.Interface_var_IsTutorial`)))

(fn `Interface_func_GetStoryArray`
  (returns (NewParam :type "Array of /Game/Structures/NPC_StoryNode_ArrayStructure Structure"))
  (return (`self.Interface_var_ArrayOfStoryNodes`)))

(fn `Interface_func_InitStoryNodeManager`
  (params (Input_var_StoryNodeArray :type "Array of /Game/Structures/NPC_StoryNode_ArrayStructure Structure (by ref)"))
  ;[1 1 1] CurrentNode starts at index 0
  (set `self.Interface_var_ArrayOfStoryNodes` Input_var_StoryNodeArray)
  (set `self.Interface_var_CurrentStoryNode` (`|GetArrayItem` Input_var_StoryNodeArray))
  (set `self.Interface_var_CurrentStoryNodeIndex` 0))

(fn `Interface_func_NewSetChildOptionAttractiveness`
  (params (Input_ChildOptions :type "Array of /Game/Structures/Story_OptionAttractiveness_pair Structure"))
  (returns (Output_ChildOptionsWithAttractivenessValues :type "Array of /Game/Structures/Story_OptionAttractiveness_pair Structure") (Output_MultipleOptions :type Boolean))
  (locals (NewLocalVar_0 :type "/Game/Structures/NPC_TraitValue_Pair Structure") (Interface_tempVar_OutputArray :type "Array of /Game/Structures/Story_OptionAttractiveness_pair Structure"))
  (bind _returnvalue (`KismetArrayLibrary.Array_Length` Input_ChildOptions))
  (bind _interface_tempvar_outputarray (`local.Interface_tempVar_OutputArray`))
  (`KismetArrayLibrary.Array_Resize` (`local.Interface_tempVar_OutputArray`) _returnvalue)
  (if (> _returnvalue 1)
    (bind _output_get (set `local.Interface_tempVar_OutputArray` Input_ChildOptions))
    (for (_array_element _array_index) _output_get
      (for _array_element_2 (`.Node_ApplicableTraits_22_6354D9CD4E436EBECE18DEA3AFC86B0E` (break `/Game/Structures/NPC_StoryNode_ArrayStructure` (`.Option_2_889744D94C7D03322B8659A176F6ADAD` (break `/Game/Structures/Story_OptionAttractiveness_pair` _array_element))))
        (for _array_element_3 (`.Structure_NPC_TRAITS_23_7CB29F7A47A8C68CF2097EAB3D998E8E` (break `/Game/Structures/NPC_Structure` (`self.Interface_var_CurrentNPCArrayStructure`)))
          (bind (_structure_traitname _structure_traitvalue) (break `/Game/Structures/NPC_TraitValue_Pair` _array_element_3))
          (bind (_structure_traitname_2 _structure_traitvalue_2) (break `/Game/Structures/NPC_TraitValue_Pair` _array_element_2))
          (if (== _structure_traitname _structure_traitname_2)
            (bind _output_attractivenessvaluetoadd (`self.Interface_func_CalculateAttractivenessToAdd` _structure_traitvalue _structure_traitvalue_2))
            (bind (_option _attractiveness) (break `/Game/Structures/Story_OptionAttractiveness_pair` _array_element))
            (`KismetArrayLibrary.Array_Set` (`local.Interface_tempVar_OutputArray`) _array_index (make `/Game/Structures/Story_OptionAttractiveness_pair` _option (+ _attractiveness _output_attractivenessvaluetoadd)) true)))))
    (return (`local.Interface_tempVar_OutputArray`) true)
    (else
      (`KismetArrayLibrary.Array_Set` _interface_tempvar_outputarray 0 (`|GetArrayItem` Input_ChildOptions) true)
      (return _interface_tempvar_outputarray false))))

(fn `Interface_func_OpenUI`
  (params (`Input NPC Structure` :type "/Game/Structures/NPC_Structure Structure") (`Input StoryNode Array` :type "Array of /Game/Structures/NPC_StoryNode_ArrayStructure Structure (by ref)"))
  (bind _returnvalue (`GameplayStatics.GetPlayerController` 0))
  (bind _interface_var_menuref (`self.Interface_var_MenuRef`))
  (set `self.Interface_var_CurrentNPCArrayStructure` `Input NPC Structure`)
  (`self.Interface_func_InitStoryNodeManager` `Input StoryNode Array`)
  (`Widget.SetVisibility` _interface_var_menuref "Visible")
  (`WidgetBlueprintLibrary.SetInputMode_UIOnlyEx` _returnvalue _interface_var_menuref)
  (set `PlayerController.bShowMouseCursor` true _returnvalue)
  (`/Game/JSON_DEMO/Widgets/UI_StoryScreen_WBP.UI_func_InitVarFromInterface` _interface_var_menuref self))

(fn `Interface_func_SelectNextNodeFromChildren`
  (returns (OutputBool_IsGoalNode :type Boolean) (Output_CurrentStoryNode :type "/Game/Structures/NPC_StoryNode_ArrayStructure Structure"))
  (locals (Interface_tempVar_OptionAttractivenessArray :type "Array of /Game/Structures/Story_OptionAttractiveness_pair Structure") (Interface_tempVar_AttractivenessArray :type "Array of Float (double-precision)") (Interface_tempVar_BestOptionSoFar :type "/Game/Structures/Story_OptionAttractiveness_pair Structure"))
  (bind (_node_name _node_id _node_storyarc _node_story_path _isgoalnode _node_description _node_applicabletraits _node_storyoptionids) (break `/Game/Structures/NPC_StoryNode_ArrayStructure` (`self.Interface_var_CurrentStoryNode`)))
  ;[1 1 1] Make Array of Child Option Nodes
  (`KismetArrayLibrary.Array_Resize` (`local.Interface_tempVar_OptionAttractivenessArray`) (`KismetArrayLibrary.Array_Length` _node_storyoptionids))
  (for (_array_element _array_index) _node_storyoptionids
    (`KismetArrayLibrary.Array_Set` (`local.Interface_tempVar_OptionAttractivenessArray`) _array_index (make `/Game/Structures/Story_OptionAttractiveness_pair` (`|GetArrayItem` (`self.Interface_var_ArrayOfStoryNodes`) _array_element)) true))
  (bind (_output_childoptionswithattractivenessvalues _output_multipleoptions) (`self.Interface_func_NewSetChildOptionAttractiveness` (`local.Interface_tempVar_OptionAttractivenessArray`)))
  (if _output_multipleoptions
    ;[1 1 1] Find Best Option So Far, IE, the Option with the Highest Attractiveness Value
    (bind _output_get (set `local.Interface_tempVar_BestOptionSoFar` (`|GetArrayItem` _output_childoptionswithattractivenessvalues)))
    (for _array_element_2 _output_childoptionswithattractivenessvalues
      (if (> (`.Attractiveness_5_F389E8FA42EDD0A6C56C91928CDF23BF` (break `/Game/Structures/Story_OptionAttractiveness_pair` _array_element_2)) (`.Attractiveness_5_F389E8FA42EDD0A6C56C91928CDF23BF` (break `/Game/Structures/Story_OptionAttractiveness_pair` _output_get)))
        (set `local.Interface_tempVar_BestOptionSoFar` _array_element_2)))
    ;[1 1 1] Set the Best so Far as the New Current Node and return the Bool
    (bind _output_get_2 (set `self.Interface_var_CurrentStoryNode` (`.Option_2_889744D94C7D03322B8659A176F6ADAD` (break `/Game/Structures/Story_OptionAttractiveness_pair` (`local.Interface_tempVar_BestOptionSoFar`)))))
    (return (`.isGoalNODE_26_7193EA41499BC2E4A1A24485BE183C57` (break `/Game/Structures/NPC_StoryNode_ArrayStructure` _output_get_2)) (`self.Interface_var_CurrentStoryNode`))
    (else
      ;[1 1 1] Sanity Check When there is only one option
      (bind _output_get_3 (set `self.Interface_var_CurrentStoryNode` (`.Option_2_889744D94C7D03322B8659A176F6ADAD` (break `/Game/Structures/Story_OptionAttractiveness_pair` (`|GetArrayItem` _output_childoptionswithattractivenessvalues)))))
      (return (`.isGoalNODE_26_7193EA41499BC2E4A1A24485BE183C57` (break `/Game/Structures/NPC_StoryNode_ArrayStructure` _output_get_3)) (`self.Interface_var_CurrentStoryNode`)))))

(fn `Interface_func_SetChildOptionAttractiveness`
  (params (Input_ChildOptions :type "Array of /Game/Structures/Story_OptionAttractiveness_pair Structure"))
  (locals (Interface_tempVar_CurrentOptionAttractivenessPair :type "/Game/Structures/Story_OptionAttractiveness_pair Structure") (Interface_tempVar_CurrentNPCTrait :type "/Game/Structures/NPC_TraitValue_Pair Structure"))
  (bind (_option _attractiveness) (break `/Game/Structures/Story_OptionAttractiveness_pair` (`local.Interface_tempVar_CurrentOptionAttractivenessPair`)))
  ;[1 1 1] Code That Doesnt Work
  ;;[1 1 1] For Each possible Option that is in the OptionAttractiveness Array
  (for _array_element Input_ChildOptions
    (bind _output_get (set `local.Interface_tempVar_CurrentOptionAttractivenessPair` _array_element))
    ;;[1 1 1] Loop for Every Trait the NPC has
    (for _array_element_2 (`.Structure_NPC_TRAITS_23_7CB29F7A47A8C68CF2097EAB3D998E8E` (break `/Game/Structures/NPC_Structure` (`self.Interface_var_CurrentNPCArrayStructure`)))
      (bind _output_get_2 (set `local.Interface_tempVar_CurrentNPCTrait` _array_element_2))
      ;;[1 1 1] Loop For every Applicable trait in the current Node being examined
      (for _array_element_3 (`.Node_ApplicableTraits_22_6354D9CD4E436EBECE18DEA3AFC86B0E` (break `/Game/Structures/NPC_StoryNode_ArrayStructure` (`.Option_2_889744D94C7D03322B8659A176F6ADAD` (break `/Game/Structures/Story_OptionAttractiveness_pair` _output_get))))
        (bind (_structure_traitname _structure_traitvalue) (break `/Game/Structures/NPC_TraitValue_Pair` _array_element_3))
        (bind (_structure_traitname_2 _structure_traitvalue_2) (break `/Game/Structures/NPC_TraitValue_Pair` _output_get_2))
        ;;[1 1 1] If Trait Names equal We do calculation, otherwise we skip
        (if (`KismetStringLibrary.EqualEqual_StrStr` _structure_traitname _structure_traitname_2)
          ;;[1 1 1] Calculate and Add Attractiveness Score to the total Attractiveness Value of the Current Option
          (bind _output_attractivenessvaluetoadd (`self.Interface_func_CalculateAttractivenessToAdd` _structure_traitvalue_2 _structure_traitvalue))
          (set `local.Interface_tempVar_CurrentOptionAttractivenessPair` (make `/Game/Structures/Story_OptionAttractiveness_pair` _option (+ _attractiveness _output_attractivenessvaluetoadd)))))))
  (`KismetSystemLibrary.PrintString` "Done" true true (struct :`R` 1.0 :`B` 0.009597 :`A` 1.0) 10.0)
  (for _array_element_4 Input_ChildOptions
    (bind (_option_2 _attractiveness_2) (break `/Game/Structures/Story_OptionAttractiveness_pair` _array_element_4))
    (`KismetSystemLibrary.PrintString` (`KismetStringLibrary.Concat_StrStr` (`.Node_Name_10_EBC3BFA0408E32E988409CB23143CDA4` (break `/Game/Structures/NPC_StoryNode_ArrayStructure` _option_2)) " : " (`KismetStringLibrary.Conv_DoubleToString` _attractiveness_2)) true true (struct :`R` 1.0 :`B` 0.051108 :`A` 1.0) 10.0)))

(fn `Interface_func_SetNewTraitsForNPC`
  (params (Input_NewStructure :type "/Game/Structures/NPC_Structure Structure"))
  (set `self.Interface_var_CurrentNPCArrayStructure` Input_NewStructure))

(fn `Interface_func_SetTraitEnums`
  (bind _interface_var_alltraitnames (`self.Interface_var_AllTraitNames`))
  (bind _output_get (set `self.Interface_var_MaxTraitNumber` (`self.Interface Var Max Trait Number`)))
  (`KismetArrayLibrary.Array_Resize` _interface_var_alltraitnames _output_get)
  (`KismetArrayLibrary.Array_Set` _interface_var_alltraitnames 0 "Aggression" true)
  (`KismetArrayLibrary.Array_Set` _interface_var_alltraitnames 1 "Caution" true)
  (`KismetArrayLibrary.Array_Set` _interface_var_alltraitnames 2 "Bravery" true)
  (`KismetArrayLibrary.Array_Set` _interface_var_alltraitnames 3 "Honesty" true)
  (`KismetArrayLibrary.Array_Set` _interface_var_alltraitnames 4 "Lawfulness" true)
  (`KismetArrayLibrary.Array_Set` _interface_var_alltraitnames 5 "Kindness" true)
  (`KismetArrayLibrary.Array_Set` _interface_var_alltraitnames 6 "Generosity" true)
  (`KismetArrayLibrary.Array_Set` _interface_var_alltraitnames 7 "Charisma" true)
  (`KismetArrayLibrary.Array_Set` _interface_var_alltraitnames 8 "Brawn" true)
  (`KismetArrayLibrary.Array_Set` _interface_var_alltraitnames 9 "Agility" true)
  (`KismetArrayLibrary.Array_Set` _interface_var_alltraitnames 10 "Intelligence" true))

(fn `Interface_func_UpdateNPCFromMenu`
  (params (NPC_var_NPCJSONStructure :type "/Game/Structures/NPC_Structure Structure"))
  (`/Game/JSON_DEMO/Blueprints/Interactable_NPC_BP_v3.NPC_func_UpdateNPCFromInterface` (`self.Interface_var_CurrentNPCRef`) NPC_var_NPCJSONStructure))

(fn `UserConstructionScript`)