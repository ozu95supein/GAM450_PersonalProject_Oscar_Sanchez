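; Interactable NPC for a JSON-driven story demo that shows a "Press E" prompt and registers itself with the third-person player while they overlap its collision box.
; On BeginPlay it finds the UI interface actor, then loads its identity and traits from a JSON file.
; It builds story nodes by merging three JSON files (info, traits, options) keyed by numbered node names until a lookup fails.
; Pressing E passes both to the interface's UI.
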(event `self.ReceiveBeginPlay`
  (`self.NPC_func_InitNPC`))

(event `self.CollisionBox.OnComponentBeginOverlap`
  (params (OverlappedComponent :type "PrimitiveComponent Object Reference") (OtherActor :type "Actor Object Reference") (OtherComp :type "PrimitiveComponent Object Reference") (OtherBodyIndex :type Integer) (bFromSweep :type Boolean) (SweepResult :type "HitResult Structure (by ref)"))
  (bind _asbp_third_person_character (cast `/Game/ThirdPerson/Blueprints/BP_ThirdPersonCharacter` OtherActor))
  (`SceneComponent.SetVisibility` (`self.PressEText`) true false)
  (set `self.NPC_var_PlayerIsNear` true)
  (`/Game/ThirdPerson/Blueprints/BP_ThirdPersonCharacter.Player_func_NPCIsNear` _asbp_third_person_character self))

(event `self.CollisionBox.OnComponentEndOverlap`
  (params (OverlappedComponent :type "PrimitiveComponent Object Reference") (OtherActor :type "Actor Object Reference") (OtherComp :type "PrimitiveComponent Object Reference") (OtherBodyIndex :type Integer))
  (bind _asbp_third_person_character (cast `/Game/ThirdPerson/Blueprints/BP_ThirdPersonCharacter` OtherActor))
  (`SceneComponent.SetVisibility` (`self.PressEText`) false false)
  (set `self.NPC_var_PlayerIsNear` false)
  (`/Game/ThirdPerson/Blueprints/BP_ThirdPersonCharacter.Player_func_NPCIsNoLongerNear` _asbp_third_person_character))

(fn `NPC_func_ConvertOptionsJsonToOptionsIntArray`
  (params (InputJson :type "JsonObjectWrapper Structure"))
  (returns (OutputArray :type "Array of Integer"))
  (locals (NPC_tempVar_ArrayOfOptionInts :type "Array of Integer") (NPC_tempVar_IntCounter :type Integer) (NPC_tempVar_WhileRunningBool :type Boolean))
  (bind _npc_tempvar_intcounter (`local.NPC_tempVar_IntCounter`))
  (bind _npc_tempvar_arrayofoptionints (`local.NPC_tempVar_ArrayOfOptionInts`))
  ;[1 1 1] Prepare Temp vars and set up
  (`KismetArrayLibrary.Array_Resize` (`local.NPC_tempVar_ArrayOfOptionInts`) 4)
  (set `local.NPC_tempVar_WhileRunningBool` true)
  (set `local.NPC_tempVar_IntCounter` 0)
  ;[1 1 1] Loop through the current options that are present inside the JSON
  (while (`local.NPC_tempVar_WhileRunningBool`)
    (bind (_outvalue _returnvalue) (`|GetJsonField` InputJson (`KismetStringLibrary.Concat_StrStr` "OPTION_" (`KismetStringLibrary.Conv_IntToString` (`local.NPC_tempVar_IntCounter`)))))
    ;[1 1 1] Set an element in the output array and increment the counter
    (if _returnvalue
      (`KismetArrayLibrary.Array_Set` (`local.NPC_tempVar_ArrayOfOptionInts`) _npc_tempvar_intcounter _outvalue true)
      (`/Engine/EditorBlueprintResources/StandardMacros.IncrementInt` _npc_tempvar_intcounter)
      (else
        (set `local.NPC_tempVar_WhileRunningBool` false))))
  (`KismetArrayLibrary.Array_Resize` _npc_tempvar_arrayofoptionints (`local.NPC_tempVar_IntCounter`))
  (return _npc_tempvar_arrayofoptionints))

(fn `NPC_func_ConvertTraitJsonToTraitArray`
  (params (InputTraitJson :type "JsonObjectWrapper Structure"))
  (returns (OutputTraitArray :type "Array of /Game/Structures/NPC_TraitValue_Pair Structure"))
  (locals (NPC_tempVar_TraitArray :type "Array of /Game/Structures/NPC_TraitValue_Pair Structure") (NPC_tempVar_Counter :type Integer))
  (bind _npc_tempvar_traitarray (`local.NPC_tempVar_TraitArray`))
  (bind _fieldnames (`JsonBlueprintFunctionLibrary.GetFieldNames` InputTraitJson)) ; get all the trait field names in traits JSON
  ;[1 1 1] Prep the Temp Trait Array and resize/clear
  (`KismetArrayLibrary.Array_Resize` _npc_tempvar_traitarray (`KismetArrayLibrary.Array_Length` _fieldnames))
  (`KismetArrayLibrary.Array_Clear` _npc_tempvar_traitarray)
  ;[1 1 1] For Every Trait, create a trait value pair
  (for (_array_element _array_index) _fieldnames
    (bind (_outvalue _returnvalue) (`|GetJsonField` InputTraitJson _array_element))
    (if _returnvalue
      (`KismetArrayLibrary.Array_Set` (`local.NPC_tempVar_TraitArray`) _array_index (make `/Game/Structures/NPC_TraitValue_Pair` _array_element _outvalue) true)))
  (return (`local.NPC_tempVar_TraitArray`)))

(fn `NPC_func_InitNPC`
  (bind _returnvalue (`GameplayStatics.GetActorOfClass` "/Game/JSON_DEMO/Blueprints/NPC_UI_Interface_BP_v2.NPC_UI_Interface_BP_v2_C"))
  (bind _output_get (set `self.NPC_var_InterfaceRef` _returnvalue))
  (`/Game/JSON_DEMO/Blueprints/NPC_UI_Interface_BP_v2.Interface_func_SetTraitEnums` _output_get)
  (set `self.NPC_var_PlayerIsNear` false)
  (`SceneComponent.SetVisibility` (`self.PressEText`) false false)
  (`self.NPC_func_LoadNPCJSON`)
  (`self.NPC_func_LoadStoryJSON`))

(fn `NPC_func_LoadNPCJSON`
  (bind (_outjsonobject _returnvalue) (`JsonBlueprintFunctionLibrary.FromFile` (make `FilePath` (`KismetStringLibrary.Concat_StrStr` (`BlueprintPathsLibrary.ProjectContentDir`) "\\JSONs\\" (`self.NPC_var_NPCJSONString`)))))
  (if _returnvalue
    (`KismetArrayLibrary.Array_Resize` (`self.NPC_tempVar_TempTraitArray`) (`/Game/JSON_DEMO/Blueprints/NPC_UI_Interface_BP_v2.Interface_var_MaxTraitNumber` (`self.NPC_var_InterfaceRef`)))
    ;[1 1 1] Get each JSON field before gettin the array
    (bind _outvalue (`|GetJsonField` _outjsonobject "NPC_ID"))
    (bind _outvalue_2 (`|GetJsonField` _outjsonobject "NPC_NAME"))
    (bind _outvalue_3 (`|GetJsonField` _outjsonobject "NPC_StoryIntroDuction"))
    (bind _outvalue_4 (`|GetJsonField` _outjsonobject "NPC_TRAITS"))
    (bind _fieldnames (`JsonBlueprintFunctionLibrary.GetFieldNames` _outvalue_4))
    (for (_array_element _array_index) _fieldnames
      ;[1 1 1] Loop Body to print and set Keyvalue pairs
      (bind _outvalue_5 (`|GetJsonField` _outvalue_4 _array_element))
      (`KismetArrayLibrary.Array_Set` (`self.NPC_tempVar_TempTraitArray`) _array_index (make `/Game/Structures/NPC_TraitValue_Pair` _array_element _outvalue_5) true))
    ;[1 1 1] Making and Setting the final JSON Structure for the NPC
    (set `self.NPC_var_NPCJSONStructure` (make `/Game/Structures/NPC_Structure` _outvalue _outvalue_2 (`self.NPC_tempVar_TempTraitArray`) _outvalue_3))))

(fn `NPC_func_LoadStoryJSON`
  (bind _npc_tempvar_tempoptionsarray (`self.NPC_tempVar_TempOptionsArray`))
  (bind _npc_tempvar_temptraitarray (`self.NPC_tempVar_TempTraitArray`))
  (bind _returnvalue (`KismetStringLibrary.Concat_StrStr` "node" (`KismetStringLibrary.Conv_IntToString` (`self.NPC_var_NodeCounter`))))
  ;[1 1 1] Prep other things, PLEASE NOTE THE DEFAULT SIZE of the story node array may or may not be final size
  (`KismetArrayLibrary.Array_Resize` (`self.NPC_var_ArrayOfStoryNodes`) (`self.NPC_var_DefaultSizeOfStoryNodeArray`))
  (set `self.NPC_var_NodeCounter` 0)
  (set `self.NPC_tempVar_LoopRunnin` true)
  ;[1 1 1] Load each separate JSON File
  (`|ExecutionSequence`
    (:`then_0`
      (bind _outjsonobject (`JsonBlueprintFunctionLibrary.FromFile` (make `FilePath` (`KismetStringLibrary.Concat_StrStr` (`BlueprintPathsLibrary.ProjectContentDir`) "\\JSONs\\" (`self.NPC_var_StoryNodeInfoJSONString`))))) ; StoryNodeInfo
    )
    (:`then_1`
      (bind _outjsonobject_2 (`JsonBlueprintFunctionLibrary.FromFile` (make `FilePath` (`KismetStringLibrary.Concat_StrStr` (`BlueprintPathsLibrary.ProjectContentDir`) "\\JSONs\\" (`self.NPC_var_StoryNodeTraitsJsonString`))))) ; StoryNodeTraits
    )
    (:`then_2`
      (bind _outjsonobject_3 (`JsonBlueprintFunctionLibrary.FromFile` (make `FilePath` (`KismetStringLibrary.Concat_StrStr` (`BlueprintPathsLibrary.ProjectContentDir`) "\\JSONs\\" (`self.NPC_var_StoryNodeOptionsJsonString`))))) ; StoryNodeOptions
    )
    (:`then_3`
      ;[1 1 1] Begin loop and go through each JSON and use them to create final Structure
      (while (`self.NPC_tempVar_LoopRunnin`)
        (`|ExecutionSequence`
          (:`then_0`
            (bind (_outvalue _returnvalue_2) (`|GetJsonField` _outjsonobject _returnvalue))
            ;[1 1 1] End while loop if we cant get a field
            (if (not _returnvalue_2)
              (`KismetSystemLibrary.PrintString` (`KismetStringLibrary.Concat_StrStr` "Failure to find Field: " _returnvalue) false true (struct :`R` 1.0 :`G` 0.004658 :`A` 1.0) 10.0)
              (set `self.NPC_tempVar_LoopRunnin` false)))
          (:`then_1`
            (bind _outvalue_2 (`|GetJsonField` _outjsonobject_2 _returnvalue))
            (bind _fieldnames (`JsonBlueprintFunctionLibrary.GetFieldNames` _outvalue_2))
            ;[1 1 1] clear and resize the temp trait array
            (`KismetArrayLibrary.Array_Resize` _npc_tempvar_temptraitarray (`KismetArrayLibrary.Array_Length` _fieldnames))
            (`KismetArrayLibrary.Array_Clear` _npc_tempvar_temptraitarray)
            ;[1 1 1] Loop Through the trait fields and pass the values to the temp trait array
            (for (_array_element _array_index) _fieldnames
              (bind _outvalue_3 (`|GetJsonField` _outvalue_2 _array_element))
              (`KismetArrayLibrary.Array_Set` (`self.NPC_tempVar_TempTraitArray`) _array_index (make `/Game/Structures/NPC_TraitValue_Pair` _array_element _outvalue_3) true)))
          (:`then_2`
            (bind _outvalue_4 (`|GetJsonField` _outjsonobject_3 _returnvalue))
            (bind _fieldnames_2 (`JsonBlueprintFunctionLibrary.GetFieldNames` _outvalue_4))
            ;[1 1 1] clear and resize the temp trait array
            (`KismetArrayLibrary.Array_Resize` _npc_tempvar_tempoptionsarray (`KismetArrayLibrary.Array_Length` _fieldnames_2))
            (`KismetArrayLibrary.Array_Clear` _npc_tempvar_tempoptionsarray)
            ;[1 1 1] Loop Through the trait fields and pass the values to the temp trait array
            (for (_array_element_2 _array_index_2) _fieldnames_2
              (bind _outvalue_5 (`|GetJsonField` _outvalue_4 _array_element_2))
              (`KismetArrayLibrary.Array_Set` (`self.NPC_tempVar_TempOptionsArray`) _array_index_2 _outvalue_5 true)))
          (:`then_3`
            (bind (_node_name _node_id _node_storyarc _node_story_path _isgoalnode _node_description) (break `/Game/Structures/StoryNodeInfo_Structure` _outvalue))
            (`KismetArrayLibrary.Array_Set` (`self.NPC_var_ArrayOfStoryNodes`) (`self.NPC_var_NodeCounter`) (make `/Game/Structures/NPC_StoryNode_ArrayStructure` _node_name _node_id _node_storyarc _node_story_path _isgoalnode _node_description (`self.NPC_tempVar_TempTraitArray`) (`self.NPC_tempVar_TempOptionsArray`)) true)
            (`/Engine/EditorBlueprintResources/StandardMacros.IncrementInt` (`self.NPC_var_NodeCounter`)))))
      (`KismetSystemLibrary.PrintString` "COMPLETE" false false (struct :`R` 1.0 :`G` 0.011368 :`A` 1.0) 10.0))))

(fn `NPC_func_PlayerPressedE`
  (`/Game/JSON_DEMO/Blueprints/NPC_UI_Interface_BP_v2.Interface_func_OpenUI` (`self.NPC_var_InterfaceRef`) (`self.NPC_var_NPCJSONStructure`) (`self.NPC_var_ArrayOfStoryNodes`)))

(fn `NPC_func_UpdateNPCFromInterface`
  (params (NPC_var_NPCJSONStructure :type "/Game/Structures/NPC_Structure Structure"))
  (set `self.NPC_var_NPCJSONStructure` NPC_var_NPCJSONStructure))

(fn `UserConstructionScript`)