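; Interactable NPC for a JSON demo that loads its identity, traits and story from files and lets the player talk to it.
; On BeginPlay it builds an NPC struct from one JSON file and fills a story node list by reading sequentially numbered node fields from another.
; Its collision box toggles the press-E prompt and notifies the player character.
; OpenConversationMenu passes the struct and itself to the UI manager.
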(event `self.ReceiveBeginPlay`
  (`self.InitNPCFromJSON`)
  (`self.LoadStoryNodesFromJson`))

(event `self.CollisionBox.OnComponentBeginOverlap`
  (params (OverlappedComponent :type "PrimitiveComponent Object Reference") (OtherActor :type "Actor Object Reference") (OtherComp :type "PrimitiveComponent Object Reference") (OtherBodyIndex :type Integer) (bFromSweep :type Boolean) (SweepResult :type "HitResult Structure (by ref)"))
  (bind _asbp_third_person_character (cast `/Game/ThirdPerson/Blueprints/BP_ThirdPersonCharacter` OtherActor))
  (`SceneComponent.SetVisibility` (`self.PressEText`) true false)
  (set `self.PlayerIsNear` true)
  (`/Game/ThirdPerson/Blueprints/BP_ThirdPersonCharacter.NPC_Is_Nearby_To_Talk` _asbp_third_person_character self))

(event `self.CollisionBox.OnComponentEndOverlap`
  (params (OverlappedComponent :type "PrimitiveComponent Object Reference") (OtherActor :type "Actor Object Reference") (OtherComp :type "PrimitiveComponent Object Reference") (OtherBodyIndex :type Integer))
  (bind _asbp_third_person_character (cast `/Game/ThirdPerson/Blueprints/BP_ThirdPersonCharacter` OtherActor))
  (`SceneComponent.SetVisibility` (`self.PressEText`) false false)
  (set `self.PlayerIsNear` false)
  (`/Game/ThirdPerson/Blueprints/BP_ThirdPersonCharacter.NPC_Is_No_Longer_Nearby` _asbp_third_person_character))

(fn `DisplayInteractText`)

(fn `DisplayNPCInfo`
  (locals (NPC_JSON_OBJ :type "JsonObjectWrapper Structure") (NewLocalVar_0 :type String)))

(fn `InitNPCFromJSON`
  (bind _returnvalue (`KismetStringLibrary.Concat_StrStr` (`BlueprintPathsLibrary.ProjectContentDir`) "\\JSONs\\" (`self.JSON_TO_LOAD`)))
  (set `self.PlayerIsNear` false)
  (`SceneComponent.SetVisibility` (`self.PressEText`) false false)
  (`KismetSystemLibrary.PrintString` _returnvalue false true (struct :`R` 1.0 :`G` 0.186423 :`A` 1.0) 50.0)
  (bind (_outjsonobject _returnvalue_2) (`JsonBlueprintFunctionLibrary.FromFile` (make `FilePath` _returnvalue)))
  (if _returnvalue_2
    (`KismetArrayLibrary.Array_Resize` (`self.TempTraitValuePairArray`) 11)
    ;[1 1 1] Get each JSON field before gettin the array
    (bind _outvalue (`|GetJsonField` _outjsonobject "NPC_ID"))
    (bind _outvalue_2 (`|GetJsonField` _outjsonobject "NPC_NAME"))
    (bind _outvalue_3 (`|GetJsonField` _outjsonobject "NPC_StoryIntroDuction"))
    (bind _outvalue_4 (`|GetJsonField` _outjsonobject "NPC_TRAITS"))
    (bind _fieldnames (`JsonBlueprintFunctionLibrary.GetFieldNames` _outvalue_4))
    (for (_array_element _array_index) _fieldnames
      ;[1 1 1] Loop Body to print and set Keyvalue pairs
      (bind _outvalue_5 (`|GetJsonField` _outvalue_4 _array_element))
      (`KismetSystemLibrary.PrintString` (`KismetStringLibrary.Concat_StrStr` _array_element " : " (`KismetStringLibrary.Conv_DoubleToString` _outvalue_5)) false true (struct :`G` 0.66 :`B` 1.0 :`A` 1.0) 10.0)
      (`KismetArrayLibrary.Array_Set` (`self.TempTraitValuePairArray`) _array_index (make `/Game/Structures/NPC_TraitValue_Pair` _array_element _outvalue_5)))
    ;[1 1 1] Making and Setting the final JSON Structure for the NPC
    (set `self.NPC_JSON_STRUCTURE` (make `/Game/Structures/NPC_Structure` _outvalue _outvalue_2 (`self.TempTraitValuePairArray`) _outvalue_3))
    (else
      (`KismetSystemLibrary.PrintString` "FailToLoad:" false true (struct :`G` 0.66 :`B` 1.0 :`A` 1.0) 10.0)
      (`KismetSystemLibrary.PrintString` _returnvalue false true (struct :`G` 0.66 :`B` 1.0 :`A` 1.0) 10.0))))

(fn `LoadStoryNodesFromJson`
  (bind _returnvalue (`KismetStringLibrary.Concat_StrStr` (`BlueprintPathsLibrary.ProjectContentDir`) "\\JSONs\\" (`self.STORY_JSON_TO_LOAD`)))
  (set `self.NodeCounter` 0)
  (set `self.LoopRunnin` true)
  (`KismetSystemLibrary.PrintString` _returnvalue false true (struct :`R` 1.0 :`G` 0.186423 :`A` 1.0) 50.0)
  (bind (_outjsonobject _returnvalue_2) (`JsonBlueprintFunctionLibrary.FromFile` (make `FilePath` _returnvalue)))
  (if _returnvalue_2
    (while (`self.LoopRunnin`)
      (bind (_outvalue _returnvalue_3) (`|GetJsonField` _outjsonobject (`KismetStringLibrary.Concat_StrStr` "node" (`KismetStringLibrary.Conv_IntToString` (`self.NodeCounter`)))))
      (if _returnvalue_3
        (bind (_node_name _node_id _node_storyarc _node_story_path _node_isgoalnode _node_description _node_applicabletraits _node_storyoptionids) (break `/Game/Structures/NPC_StoryNode_Structure` _outvalue))
        (`KismetArrayLibrary.Array_Set` (`self.NPC_StoryNodes_List`) (`self.NodeCounter`) (make `/Game/Structures/NPC_StoryNode_Structure` _node_name _node_id _node_storyarc _node_story_path _node_isgoalnode _node_description _node_applicabletraits _node_storyoptionids) true)
        (`/Engine/EditorBlueprintResources/StandardMacros.IncrementInt` (`self.NodeCounter`))
        (else
          (set `self.LoopRunnin` false))))
    (`KismetSystemLibrary.PrintString` "Complete Loop")
    (`KismetSystemLibrary.PrintString` (`KismetStringLibrary.Concat_StrStr` "Size of Array is: " (`KismetStringLibrary.Conv_IntToString` (`KismetArrayLibrary.Array_Length` (`self.NPC_StoryNodes_List`)))))
    (else
      (`KismetSystemLibrary.PrintString` "FAIL"))))

(fn `OpenConversationMenu`
  (`/Game/JSON_DEMO/Blueprints/NPC_UI_Interface_BP.Open_Conversation_Menu` (`self.UI_Manager`) (`self.NPC_JSON_STRUCTURE`) self))

(fn `PlayerPressedEButton`)

(fn `UpdateNPC_with_NewJSONObject`
  (params (NPC_JSON_STRUCTURE :type "/Game/Structures/NPC_Structure Structure"))
  (set `self.NPC_JSON_STRUCTURE` NPC_JSON_STRUCTURE))

(fn `UserConstructionScript`)