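; Interactable NPC whose identity, traits and story nodes are data-driven from JSON files, for conversations with the player.
; On BeginPlay it finds the UI interface actor, then loads both files from Content/JSONs into structs, reading sequential "nodeN" fields until one is missing.
; Its collision box toggles the "Press E" prompt and registers or clears it as the character's nearby NPC.
; The PlayerPressedE function opens the UI through that interface actor.
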(event `self.ReceiveBeginPlay`
  (`self.NPC_func_InitNPC`))

(event `self.CollisionBox.OnComponentBeginOverlap`
  (params (OverlappedComponent :type "PrimitiveComponent Object Reference") (OtherActor :type "Actor Object Reference") (OtherComp :type "PrimitiveComponent Object Reference") (OtherBodyIndex :type Integer) (bFromSweep :type Boolean) (SweepResult :type "HitResult Structure (by ref)"))
  (bind _asbp_third_person_character (cast `/Game/ThirdPerson/Blueprints/BP_ThirdPersonCharacter` OtherActor))
  (`SceneComponent.SetVisibility` (`self.PressEText`) true false)
  (set `self.NPC_var_PlayerIsNear` true)
  (`/Game/ThirdPerson/Blueprints/BP_ThirdPersonCharacter.NPC_Is_Nearby_To_Talk` _asbp_third_person_character null self))

(event `self.CollisionBox.OnComponentEndOverlap`
  (params (OverlappedComponent :type "PrimitiveComponent Object Reference") (OtherActor :type "Actor Object Reference") (OtherComp :type "PrimitiveComponent Object Reference") (OtherBodyIndex :type Integer))
  (bind _asbp_third_person_character (cast `/Game/ThirdPerson/Blueprints/BP_ThirdPersonCharacter` OtherActor))
  (`SceneComponent.SetVisibility` (`self.PressEText`) false false)
  (set `self.NPC_var_PlayerIsNear` false)
  (`/Game/ThirdPerson/Blueprints/BP_ThirdPersonCharacter.NPC_Is_No_Longer_Nearby` _asbp_third_person_character))

(fn `NPC_func_InitNPC`
  (bind _returnvalue (`GameplayStatics.GetActorOfClass` "/Game/JSON_DEMO/Blueprints/NPC_UI_Interface_BP_v2.NPC_UI_Interface_BP_v2_C"))
  (set `self.NPC_var_InterfaceRef` _returnvalue)
  (set `self.NPC_var_PlayerIsNear` false)
  (`SceneComponent.SetVisibility` (`self.PressEText`) false false)
  (`self.NPC_func_LoadNPCJSON`)
  (`self.NPC_func_LoadStoryJSON`))

(fn `NPC_func_LoadNPCJSON`
  (bind _npc_var_npcjsonstring (`self.NPC_var_NPCJSONString`))
  (bind (_outjsonobject _returnvalue) (`JsonBlueprintFunctionLibrary.FromFile` (make `FilePath` (`KismetStringLibrary.Concat_StrStr` (`BlueprintPathsLibrary.ProjectContentDir`) "\\JSONs\\" _npc_var_npcjsonstring))))
  (if _returnvalue
    (`KismetArrayLibrary.Array_Resize` (`self.NPC_var_TempTraitArray`) (`/Game/JSON_DEMO/Blueprints/NPC_UI_Interface_BP_v2.Interface_var_MaxTraitNumber` (`self.NPC_var_InterfaceRef`)))
    ;[1 1 1] Get each JSON field before gettin the array
    (bind _outvalue (`|GetJsonField` _outjsonobject "NPC_ID"))
    (bind _outvalue_2 (`|GetJsonField` _outjsonobject "NPC_NAME"))
    (bind _outvalue_3 (`|GetJsonField` _outjsonobject "NPC_StoryIntroDuction"))
    (bind _outvalue_4 (`|GetJsonField` _outjsonobject "NPC_TRAITS"))
    (bind _fieldnames (`JsonBlueprintFunctionLibrary.GetFieldNames` _outvalue_4))
    (for (_array_element _array_index) _fieldnames
      ;[1 1 1] Loop Body to print and set Keyvalue pairs
      (bind _outvalue_5 (`|GetJsonField` _outvalue_4 _array_element))
      (`KismetSystemLibrary.PrintString` (`KismetStringLibrary.Concat_StrStr` _array_element " : " (`KismetStringLibrary.Conv_DoubleToString` _outvalue_5)) false true (struct :`G` 0.66 :`B` 1.0 :`A` 1.0) 10.0)
      (`KismetArrayLibrary.Array_Set` (`self.NPC_var_TempTraitArray`) _array_index (make `/Game/Structures/NPC_TraitValue_Pair` _array_element _outvalue_5) true))
    ;[1 1 1] Making and Setting the final JSON Structure for the NPC
    (set `self.NPC_var_NPCJSONStructure` (make `/Game/Structures/NPC_Structure` _outvalue _outvalue_2 (`self.NPC_var_TempTraitArray`) _outvalue_3))
    (else
      (`KismetSystemLibrary.PrintString` "FailToLoad:" true true (struct :`G` 0.66 :`B` 1.0 :`A` 1.0) 10.0)
      (`KismetSystemLibrary.PrintString` _npc_var_npcjsonstring false true (struct :`G` 0.66 :`B` 1.0 :`A` 1.0) 10.0))))

(fn `NPC_func_LoadStoryJSON`
  (bind _returnvalue (`KismetArrayLibrary.Array_Length` (`self.NPC_var_StoryNodesArray`)))
  (bind _returnvalue_2 (`KismetStringLibrary.Concat_StrStr` (`BlueprintPathsLibrary.ProjectContentDir`) "\\JSONs\\" (`self.NPC_var_StoryJSONString`)))
  (set `self.NPC_var_NodeCounter` 0)
  (set `self.NPC_var_LoopRunnin` true)
  (`KismetSystemLibrary.PrintString` _returnvalue_2 false true (struct :`R` 1.0 :`G` 0.186423 :`A` 1.0) 50.0)
  (bind (_outjsonobject _returnvalue_3) (`JsonBlueprintFunctionLibrary.FromFile` (make `FilePath` _returnvalue_2)))
  (if _returnvalue_3
    (while (`self.NPC_var_LoopRunnin`)
      (bind (_outvalue _returnvalue_4) (`|GetJsonField` _outjsonobject (`KismetStringLibrary.Concat_StrStr` "node" (`KismetStringLibrary.Conv_IntToString` (`self.NPC_var_NodeCounter`)))))
      (if _returnvalue_4
        (bind (_node_name _node_id _node_storyarc _node_story_path _node_isgoalnode _node_description _node_applicabletraits _node_storyoptionids) (break `/Game/Structures/NPC_StoryNode_Structure` _outvalue))
        (`KismetArrayLibrary.Array_Set` (`self.NPC_var_StoryNodesArray`) (`self.NPC_var_NodeCounter`) (make `/Game/Structures/NPC_StoryNode_Structure` _node_name _node_id _node_storyarc _node_story_path _node_isgoalnode _node_description _node_applicabletraits _node_storyoptionids) true)
        (`/Engine/EditorBlueprintResources/StandardMacros.IncrementInt` (`self.NPC_var_NodeCounter`))
        (else
          (set `self.NPC_var_LoopRunnin` false))))
    (`KismetSystemLibrary.PrintString` "Complete Loop")
    (`KismetSystemLibrary.PrintString` (`KismetStringLibrary.Concat_StrStr` "Size of Array is: " (`KismetStringLibrary.Conv_IntToString` _returnvalue)))
    (set `self.NPC_var_StoryNodesNumber` _returnvalue)
    (set `self.NPC_var_CurrentStoryNode` (`|GetArrayItem` (`self.NPC_var_StoryNodesArray`)))
    (else
      (`KismetSystemLibrary.PrintString` "FAIL"))))

(fn `NPC_func_PlayerPressedE`
  (`/Game/JSON_DEMO/Blueprints/NPC_UI_Interface_BP_v2.Interface_func_OpenUI` (`self.NPC_var_InterfaceRef`) null))

(fn `UserConstructionScript`)