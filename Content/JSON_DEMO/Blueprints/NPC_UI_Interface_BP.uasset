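; NPC_UI_Interface_BP is an actor that bridges NPCs and the dialogue UI in the JSON demo.
; On BeginPlay it creates a hidden UI_MainDialogue_Widget and passes it a reference to itself.
; Opening a conversation stores the NPC, shows the widget with cursor and UI-only input, then feeds it the NPC and its story nodes.
; An update function forwards the NPC JSON structure to the current NPC Blueprint.
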(event `self.ReceiveBeginPlay`
  (`self.CreateUIMenu_from_Interface`))

(fn `CreateUIMenu_from_Interface`
  (bind _returnvalue (`|CreateWidget` "/Game/JSON_DEMO/Widgets/UI_MainDialogue_Widget.UI_MainDialogue_Widget_C" (`GameplayStatics.GetPlayerController` 0)))
  (`UserWidget.AddToViewport` _returnvalue 0)
  (`/Game/JSON_DEMO/Widgets/UI_MainDialogue_Widget.SetInterfaceVar` _returnvalue self)
  (set `self.CurrenMenu_WBP` _returnvalue)
  (`Widget.SetVisibility` _returnvalue "Hidden"))

(fn `Open_Conversation_Menu`
  (params (CurrentFocussedNPC :type "/Game/Structures/NPC_Structure Structure") (CurrentNPC_BP :type "/Game/JSON_DEMO/Blueprints/Interactable_NPC_BP Object Reference"))
  (bind _returnvalue (`GameplayStatics.GetPlayerController` 0))
  (bind _currenmenu_wbp (`self.CurrenMenu_WBP`))
  (set `self.CurrentNPC_BP` CurrentNPC_BP)
  (`Widget.SetVisibility` _currenmenu_wbp "Visible")
  (`WidgetBlueprintLibrary.SetInputMode_UIOnlyEx` _returnvalue _currenmenu_wbp)
  (set `PlayerController.bShowMouseCursor` true _returnvalue)
  (`/Game/JSON_DEMO/Widgets/UI_MainDialogue_Widget.SetNewCurrentNPC` _currenmenu_wbp CurrentFocussedNPC)
  (`/Game/JSON_DEMO/Widgets/UI_MainDialogue_Widget.Init_Menu` _currenmenu_wbp)
  (`/Game/JSON_DEMO/Widgets/UI_MainDialogue_Widget.SetNPC_StoryNodes_Array` _currenmenu_wbp (`/Game/JSON_DEMO/Blueprints/Interactable_NPC_BP.NPC_StoryNodes_List` CurrentNPC_BP)))

(fn `UpdateNPCInfoFromMenu`)

(fn `UpdateNPCJsonObject_from_UIMenu`
  (params (NPC_JSON_STRUCTURE :type "/Game/Structures/NPC_Structure Structure"))
  (`/Game/JSON_DEMO/Blueprints/Interactable_NPC_BP.UpdateNPC_with_NewJSONObject` (`self.CurrentNPC_BP`) NPC_JSON_STRUCTURE))

(fn `UserConstructionScript`)